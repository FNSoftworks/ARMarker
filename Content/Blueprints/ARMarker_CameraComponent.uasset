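; AR camera actor that starts the ARMarker plugin and displays the device camera feed on a plane.
; On BeginPlay it initializes template-matching color detection, then feeds frames into a dynamic material set for resolution and orientation.
; It also loads standard and NFT markers from enum names, and cleans up on EndPlay.
; On a first iOS run it shows a loading screen and restarts the game after a short delay.
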(event EventBeginPlay
  (bind _markers (Variables|Default|GetMarkers))
  (bind _markersnft (Variables|Default|GetMarkersNFT))
  (bind _returnvalue (Class|ARMarkerComponent|Start (Variables|Default|GetARMarker)))
  (Development|PrintString _returnvalue true true "(R=0.000000,G=0.660000,B=1.000000,A=1.000000)" 5e+01)
  (Utilities|FlowControl|Sequence
    (:then_0
      ;[1 0 0] ARMarker Camera Config
      (bind (_webcamresx _webcamresy _firstrunios _returnvalue_2) (Class|ARMarkerComponent|Init (Variables|Default|GetARMarker) false 1 (Variables|Default|GetDeviceOrientation) "TEMPLATE_MATCHING_COLOR"))
      ;;[1 1 1 0] IOS Config
      (if _firstrunios
        (Development|PrintString "iOS Started")
        (Variables|Default|SetFirstRunIOS _firstrunios)
        (bind _returnvalue_3 (UserInterface|CreateWidget "/ARMarker/UI/LoadingScreen.LoadingScreen_C"))
        (UserInterface|Viewport|AddtoViewport _returnvalue_3 0)
        (Utilities|FlowControl|Delay 0.2)
        (bind _asgame_mode (Utilities|Casting|CastToGameMode (Game|GetGameMode)))
        (Class|GameMode|RestartGame _asgame_mode)))
    (:then_1
      (Development|PrintString (Utilities|String|ToString(Boolean) _returnvalue_2))
      (if _returnvalue_2
        (bind _returnvalue_4 (Class|ARMarkerComponent|GetCameraFrame (Variables|Default|GetARMarker)))
        (bind _returnvalue_5 (Class|ARMarkerComponent|CreateDynamicMaterialInstance (Variables|Default|GetARMarker) (Variables|Default|GetCameraSurfacePlane) "/ARMarker/Assets/Materials/BaseFeedScreenNoShadow.BaseFeedScreenNoShadow"))
        (Class|ARMarkerComponent|SetTextureParameterValue (Variables|Default|GetARMarker) _returnvalue_5 _returnvalue_4 "Color")
        (Rendering|Material|SetScalarParameterValue _returnvalue_5 "CamResX" (Math|Conversions|ToFloat(Integer) _webcamresx) :!class /Script/Engine.MaterialInstanceDynamic)
        (Rendering|Material|SetScalarParameterValue _returnvalue_5 "CamResY" (Math|Conversions|ToFloat(Integer) _webcamresy) :!class /Script/Engine.MaterialInstanceDynamic)
        (switch Utilities|FlowControl|Switch|SwitchonEDeviceOrientation (Variables|Default|GetDeviceOrientation)
          (:LANDSCAPE
            (Rendering|Material|SetScalarParameterValue _returnvalue_5 "IsPortrait" 0.0 :!class /Script/Engine.MaterialInstanceDynamic))
          (:PORTRAIT
            (Rendering|Material|SetScalarParameterValue _returnvalue_5 "IsPortrait" 1.0 :!class /Script/Engine.MaterialInstanceDynamic)))
        (Development|PrintString (Utilities|String|Append (Utilities|String|ToString(Integer) _webcamresx) "x" (Utilities|String|ToString(Integer) _webcamresy)))
        (elif (not _firstrunios)
          (Development|PrintString "Webcam init error!" true true "(R=0.000000,G=0.660000,B=1.000000,A=1.000000)" 5e+01))))
    (:then_2
      ;[0.1306 1 0] Load Markers
      ;;[1 1 1 0] Load Marker
      (bind _enumvalue (|ForEachMarkers)
        (:LoopBody
          (Utilities|Array|Add _markers (Utilities|String|EnumtoString _enumvalue)))
        (:then
          (Class|ARMarkerComponent|LoadMarkers (Variables|Default|GetARMarker) _markers))))
    (:then_3
      ;;[1 1 1 0.038] Load Marker NFT
      (bind _enumvalue_2 (|ForEachMarkersNFT)
        (:LoopBody
          (Utilities|Array|Add _markersnft (Utilities|String|EnumtoString _enumvalue_2)))
        (:then
          (Class|ARMarkerComponent|LoadMarkersNFT (Variables|Default|GetARMarker) _markersnft))))))

(event EventEndPlay
  (params (EndPlayReason :type EEndPlayReason%20Enum :default "Destroyed"))
  ;[0.03467 1 0] ARMarker Cleanup
  (Class|ARMarkerComponent|Cleanup (Variables|Default|GetARMarker)))

(fn ConstructionScript)